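; BP_DollsHouse is a doll's house that requires a random set of doll part types and shows them through mesh colours.
; Once Tick finds the Checker_BP, it picks unique types from the checker's settings and tints the house meshes to match.
; CheckDolls passes only if connected parts in the Box, read via DollPartInterface, cover every allowed type and no others.
; DestroyDolls clears DollPart-tagged actors from the Box.
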(event `self.ReceiveBeginPlay`)

(event `self.ReceiveTick`
  (params (DeltaSeconds :type "Float (single-precision)"))
  (bind _meshes (`self.Meshes`))
  (if (`KismetSystemLibrary.IsValid` (`self.Checker`))
    (if (not (`self.Created`))
      (`self.RandomiseTypes`)
      (`KismetArrayLibrary.Array_Add` _meshes (`self.RoofMesh`))
      (`KismetArrayLibrary.Array_Add` _meshes (`self.DollHouseMesh`))
      (`KismetArrayLibrary.Array_Add` _meshes (`self.Light`))
      (`KismetArrayLibrary.Array_Add` _meshes (`self.Bed`))
      (`KismetArrayLibrary.Array_Add` _meshes (`self.Lamp`))
      (`self.SetColours`)
      (set `self.Created` true))
    (else
      (bind _outactors (`GameplayStatics.GetAllActorsOfClass` "/Game/Blueprints/Checker_BP.Checker_BP_C"))
      (set `self.Checker` (`KismetArrayLibrary.Array_Get` _outactors)))))

(fn `CheckDolls`
  (returns (Correct :type Boolean))
  (locals (TypesFound :type "Array of Integer"))
  (bind _allowedtypes (`self.AllowedTypes`))
  (bind _typesfound (`local.TypesFound`))
  (set `self.Checked` true)
  (for _array_element (`PrimitiveComponent.GetOverlappingComponents` (`self.Box`))
    (bind _returnvalue (`ActorComponent.GetOwner` _array_element))
    (if (`KismetSystemLibrary.DoesImplementInterface` _returnvalue "/Game/Blueprints/DollPartInterface.DollPartInterface_C")
      (bind _asdoll_part_interface (cast `/Game/Blueprints/DollPartInterface` _returnvalue))
      (bind _connected (`/Game/Blueprints/DollPartInterface.GetPartConnected` _asdoll_part_interface))
      (bind _type (`/Game/Blueprints/DollPartInterface.GetPartType` _asdoll_part_interface))
      (if _connected
        (if (`KismetArrayLibrary.Array_Contains` _allowedtypes _type)
          (if (not (`KismetArrayLibrary.Array_Contains` _typesfound _type))
            (`KismetArrayLibrary.Array_Add` _typesfound _type)
            (`KismetSystemLibrary.PrintString` "Correct Part"))
          (else
            (return false))))))
  (if (== (`KismetArrayLibrary.Array_Length` _allowedtypes) (`KismetArrayLibrary.Array_Length` _typesfound))
    (return true)
    (else
      (return false))))

(fn `DestroyDolls`
  (for _array_element (`PrimitiveComponent.GetOverlappingComponents` (`self.Box`))
    (if (`ActorComponent.ComponentHasTag` _array_element "DollPart")
      (`self.K2_DestroyActor` (`ActorComponent.GetOwner` _array_element)))))

(fn `RandomiseTypes`
  (locals (NewType :type Integer))
  (bind _checker (`self.Checker`))
  (for _ (range (`/Game/Blueprints/Checker_BP.TypeCount` _checker))
    (bind _output_get (set `local.NewType` (`KismetMathLibrary.RandomIntegerInRange` 0 (- (`KismetArrayLibrary.Array_Length` (`/Game/Blueprints/Checker_BP.TypeColours` _checker)) 1)) :!label _label))
    (if (`KismetArrayLibrary.Array_Contains` (`self.AllowedTypes`) _output_get)
      (goto _label)
      (else
        (`KismetArrayLibrary.Array_Add` (`self.AllowedTypes`) _output_get)))))

(fn `SetColours`
  (for _array_element (`self.Meshes`)
    (`MeshComponent.SetVectorParameterValueOnMaterials` _array_element "Colour" (`KismetMathLibrary.Conv_LinearColorToVector` (`KismetArrayLibrary.Array_Get` (`/Game/Blueprints/Checker_BP.TypeColours` (`self.Checker`)) (`KismetArrayLibrary.Array_Get` (`self.AllowedTypes`)))))
    (for (_array_element_2 _array_index) (`self.AllowedTypes`)
      (`MeshComponent.SetVectorParameterValueOnMaterials` (`KismetArrayLibrary.Array_Get` (`self.Meshes`) _array_index) "Colour" (`KismetMathLibrary.Conv_LinearColorToVector` (`KismetArrayLibrary.Array_Get` (`/Game/Blueprints/Checker_BP.TypeColours` (`self.Checker`)) _array_element_2))))))

(fn `UserConstructionScript`)