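; A conveyor volume that pushes physics objects inside it along a set direction.
; Every tick it gathers the components overlapping its Box and applies a force to each one that simulates physics.
; The force follows the Arrow component's forward vector scaled by ConveyerSpeed, and is not mass-compensated, so heavier objects accelerate less.
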(event `self.ReceiveTick`
  (params (DeltaSeconds :type "Float (single-precision)"))
  (for _array_element (`PrimitiveComponent.GetOverlappingComponents` (`self.Box`))
    (if (`SceneComponent.IsSimulatingPhysics` _array_element "None")
      (`PrimitiveComponent.AddForce` _array_element (* (`SceneComponent.GetForwardVector` (`self.Arrow`)) (* 1.0 (`self.ConveyerSpeed`))) "None" false))))

(fn `UserConstructionScript`)