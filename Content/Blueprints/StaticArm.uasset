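; StaticArm is a limb part that motion controllers can pick up and attach to sockets.
; On BeginPlay it creates a physics constraint at its Socket and picks a random type, tinting the mesh from Checker_BP's TypeColours.
; Pickup breaks the constraint and attaches the mesh to the grabber; Drop restores physics and constrains it to any overlapping LimbSocket component.
; Getters expose the connected state and type.
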(event `self.ReceiveBeginPlay`
  (bind _returnvalue (`AddComponent|NODE_AddPhysicsConstraintComponent-3` :`RelativeTransform` (`SceneComponent.GetRelativeTransform` (`self.Socket`))))
  (set `self.PhysicsConstraint` _returnvalue)
  (bind _outactors (`GameplayStatics.GetAllActorsOfClass` "/Game/Blueprints/Checker_BP.Checker_BP_C"))
  (bind _typecolours (`/Game/Blueprints/Checker_BP.TypeColours` (`KismetArrayLibrary.Array_Get` _outactors)))
  (bind _output_get (set `self.Type` (`KismetMathLibrary.RandomIntegerInRange` 0 (- (`KismetArrayLibrary.Array_Length` _typecolours) 1))))
  (`MeshComponent.SetVectorParameterValueOnMaterials` (`self.LimbMesh`) "Colour" (`KismetMathLibrary.Conv_LinearColorToVector` (`KismetArrayLibrary.Array_Get` _typecolours _output_get))))

(event `/Game/VirtualRealityBP/Blueprints/PickupActorInterface.Pickup`
  (params (AttachTo :type "SceneComponent Object Reference"))
  (bind _limbmesh (`self.LimbMesh`))
  (`PrimitiveComponent.SetSimulatePhysics` _limbmesh false)
  (`PhysicsConstraintComponent.BreakConstraint` (`self.PhysicsConstraint`))
  (set `self.Connected` false)
  (`SceneComponent.K2_AttachToComponent` _limbmesh AttachTo "None" "KeepWorld" "KeepWorld" "KeepWorld" false))

(event `/Game/VirtualRealityBP/Blueprints/PickupActorInterface.Drop`
  (`PrimitiveComponent.SetSimulatePhysics` (`self.LimbMesh`) true)
  (`self.K2_DetachFromActor` "KeepWorld" "KeepWorld" "KeepWorld")
  (for _array_element (`PrimitiveComponent.GetOverlappingComponents` (`self.Socket`))
    (if (`ActorComponent.ComponentHasTag` _array_element "LimbSocket")
      (`PhysicsConstraintComponent.SetConstrainedComponents` (`self.PhysicsConstraint`) (`self.LimbMesh`) "None" _array_element "None")
      (set `self.Connected` true)
      (break))))

(fn `GetPartConnected`
  (returns (Connected :type Boolean))
  (return (`self.Connected`)))

(fn `GetPartType`
  (returns (Type :type Integer))
  (return (`self.Type`)))

(fn `UserConstructionScript`)