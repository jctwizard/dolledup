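; A grabbable skeletal limb actor that motion controllers pick up and that joints onto limb sockets when released.
; BeginPlay adds a physics constraint component at the Socket's relative transform.
; Pickup disables mesh physics, breaks the constraint and attaches the root to the given component.
; Drop restores physics, detaches, and constrains LimbMesh to the first component overlapping Socket tagged LimbSocket.
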(event `self.ReceiveBeginPlay`
  (bind _returnvalue (`AddComponent|NODE_AddPhysicsConstraintComponent-3` :`RelativeTransform` (`SceneComponent.GetRelativeTransform` (`self.Socket`))))
  (set `self.PhysicsConstraint` _returnvalue))

(event `/Game/VirtualRealityBP/Blueprints/PickupActorInterface.Pickup`
  (params (AttachTo :type "SceneComponent Object Reference"))
  (`PrimitiveComponent.SetSimulatePhysics` (`self.LimbMesh`) false)
  (`PhysicsConstraintComponent.BreakConstraint` (`self.PhysicsConstraint`))
  (`SceneComponent.K2_AttachToComponent` (`self.K2_GetRootComponent`) AttachTo "None" "KeepWorld" "KeepWorld" "KeepWorld" false))

(event `/Game/VirtualRealityBP/Blueprints/PickupActorInterface.Drop`
  (bind _limbmesh (`self.LimbMesh`))
  (`PrimitiveComponent.SetSimulatePhysics` _limbmesh true)
  (`self.K2_DetachFromActor` "KeepWorld" "KeepWorld" "KeepWorld")
  (for _array_element (`PrimitiveComponent.GetOverlappingComponents` (`self.Socket`))
    (if (`ActorComponent.ComponentHasTag` _array_element "LimbSocket")
      (`PhysicsConstraintComponent.SetConstrainedComponents` (`self.PhysicsConstraint`) _limbmesh "None" _array_element "None")
      (break))))

(fn `UserConstructionScript`)