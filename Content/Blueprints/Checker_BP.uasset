(event `self.ReceiveTick`
  (params (DeltaSeconds :type "Float (single-precision)"))
  (bind _timertext (`self.TimerText`))
  (`|ExecutionSequence`
    (:`then_0`
      (bind _output_get (set `self.Timer` (- (`self.Timer`) DeltaSeconds)))
      (`TextRenderComponent.K2_SetText` (`self.TimerText`) (`KismetTextLibrary.Conv_DoubleToText` (`KismetMathLibrary.FMax` _output_get) "HalfToEven" true 2 324 0 0))
      (`TextRenderComponent.K2_SetText` (`self.ScoreText`) (`KismetTextLibrary.Conv_IntToText` (`self.Score`) true 2))
      (if (and (<= (`self.Timer`) 0.0) (not (`self.Fired`)))
        (`TextRenderComponent.K2_SetText` _timertext (`KismetTextLibrary.Conv_StringToText` "YOU'RE  \nFIRED"))
        (`TextRenderComponent.SetXScale` _timertext 1.5)
        (`TextRenderComponent.SetYScale` _timertext 1.5)
        (`AudioComponent.Play` (`self.End`) 0.0)
        (set `self.Fired` true)
        (bind _outactors (`GameplayStatics.GetAllActorsOfClass` "/Game/Blueprints/Chute.Chute_C"))
        (for _array_element _outactors
          (`self.K2_DestroyActor` _array_element))))
    (:`then_1`
      (if (`self.Grabbed`)
        (bind _output_get_2 (set `self.resettime` (+ (`self.resettime`) DeltaSeconds)))
        (if (>= _output_get_2 (`self.resetdelay`))
          (set `self.resettime` 0.0)
          (`SceneComponent.K2_SetRelativeLocation` (`self.Button_Frame1`) (0.0 0.0 0.0) false false))))))

(event `/Game/VirtualRealityBP/Blueprints/PickupActorInterface.Pickup`
  (params (AttachTo :type "SceneComponent Object Reference"))
  (if (`self.Fired`)
    (`GameplayStatics.OpenLevel` "Factory")
    (else
      (`self.CheckHouse`)
      (`SceneComponent.K2_SetRelativeLocation` (`self.Button_Frame1`) (5.0 0.0 0.0) false false)
      (set `self.Grabbed` true))))

(fn `CheckHouse`
  (for _array_element (`PrimitiveComponent.GetOverlappingActors` (`self.HouseCheck`) "/Game/Blueprints/BP_DollsHouse.BP_DollsHouse_C")
    (bind _asbp_dolls_house (cast `/Game/Blueprints/BP_DollsHouse` _array_element))
    (if (not (`/Game/Blueprints/BP_DollsHouse.Checked` _asbp_dolls_house))
      (bind _correct (`/Game/Blueprints/BP_DollsHouse.CheckDolls` _asbp_dolls_house))
      (`|ExecutionSequence`
        (:`then_0`
          (if _correct
            (`self.Correct`)
            (else
              (`self.Failed`)))
          (`/Game/Blueprints/BP_DollsHouse.DestroyDolls` _asbp_dolls_house)
          (`self.K2_DestroyActor` _asbp_dolls_house))
        (:`then_1`
          (break))))))

(fn `Correct`
  (bind _output_get (set `self.Score` (+ (`self.Score`) 1)))
  (set `self.Timer` (+ (`self.Timer`) (`self.BonusTime`)))
  (`AudioComponent.Play` (`self.Right`) 0.0)
  (if (> (/ _output_get 3) (`self.TypeCount`))
    (set `self.TypeCount` (`KismetMathLibrary.Clamp` (+ (`self.TypeCount`) 1) 0 (- (`KismetArrayLibrary.Array_Length` (`self.TypeColours`)) 1)))))

(fn `Failed`
  (set `self.Timer` (- (`self.Timer`) (`self.PenaltyTime`)))
  (`AudioComponent.Play` (`self.Wrong`) 0.0))

(fn `UserConstructionScript`)