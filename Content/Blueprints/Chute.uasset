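; Chute is a spawner actor that periodically drops a randomly chosen actor class at its own transform.
; Tick accumulates a timer and calls Spawn whenever it reaches SpawnDuration, with BeginPlay pre-filling the timer so the first spawn happens on the first tick.
; Spawn picks a random index into SpawnableActors and uses the parallel SpawnableRandomRotation flags to choose between a random rotation and the chute's own.
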(event `self.ReceiveBeginPlay`
  (set `self.SpawnTime` (`self.SpawnDuration`)))

(event `self.ReceiveTick`
  (params (DeltaSeconds :type "Float (single-precision)"))
  (bind _output_get (set `self.SpawnTime` (+ (`self.SpawnTime`) DeltaSeconds)))
  (if (>= _output_get (`self.SpawnDuration`))
    (`self.Spawn`)
    (set `self.SpawnTime` 0.0)))

(fn `Spawn`
  (locals (SpawnIndex :type Integer))
  (bind (_returnvalue_location _returnvalue_rotation _returnvalue_scale) (`KismetMathLibrary.BreakTransform` (`self.GetTransform`)))
  (bind _spawnableactors (`self.SpawnableActors`))
  (bind _output_get (set `local.SpawnIndex` (`KismetMathLibrary.RandomIntegerInRange` 0 (- (`KismetArrayLibrary.Array_Length` _spawnableactors) 1))))
  (if (`KismetArrayLibrary.Array_Get` (`self.SpawnableRandomRotation`) _output_get)
    (bind _item (`KismetArrayLibrary.Array_Get` _spawnableactors _output_get))
    (`|SpawnActorFromClass` _item (`KismetMathLibrary.MakeTransform` _returnvalue_location (`KismetMathLibrary.RandomRotator` false) _returnvalue_scale) "Undefined" "OverrideRootScale")
    (else
      (`|SpawnActorFromClass` _item (`KismetMathLibrary.MakeTransform` _returnvalue_location _returnvalue_rotation _returnvalue_scale) "Undefined" "OverrideRootScale"))))

(fn `UserConstructionScript`)